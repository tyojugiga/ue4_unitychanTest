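; Player character Blueprint for Unity-chan that handles enemy hit reactions and subtracts damage from HP.
; Capsule overlap with BP_enemy spawns an explosion, applies damage, temporarily swaps to blackened materials and briefly raises DamageFlag.
; Pressing Z clears DamageFlag2, so enemy overlaps skip the hit and re-enable it after a delay.
; Mesh overlap with BP_enemy2 flattens the mesh, deals heavier damage, then restores its scale.
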(event OnComponentBeginOverlap(Mesh)
  (params (OverlappedComponent :type Primitive%20Component%20Object%20Reference) (OtherActor :type Actor%20Object%20Reference) (OtherComp :type Primitive%20Component%20Object%20Reference) (OtherBodyIndex :type Integer) (bFromSweep :type Boolean) (SweepResult :type Hit%20Result%20Structure%20%28by%20ref%29))
  ;[1 1 1] enemy2上に落ちるとつぶれる
  (bind _asbp_enemy_2 (Utilities|Casting|CastToBP_enemy2 OtherActor))
  (Utilities|FlowControl|Delay 0.3)
  (Transformation|SetWorldScale3D (Variables|Character|GetMesh) "2.000000,2.000000,0.010000")
  (bind _asbp_unitychan (Utilities|Casting|CastToBP_unitychan (Game|Player|GetPlayerPawn 0)))
  (Game|Damage|ApplyDamage _asbp_unitychan 1e+01 0 0)
  (Utilities|FlowControl|Delay 3.0)
  (Transformation|SetWorldScale3D (Variables|Character|GetMesh) "1.000000,1.000000,1.000000"))

(event OnComponentBeginOverlap(CapsuleComponent)
  (params (OverlappedComponent :type Primitive%20Component%20Object%20Reference) (OtherActor :type Actor%20Object%20Reference) (OtherComp :type Primitive%20Component%20Object%20Reference) (OtherBodyIndex :type Integer) (bFromSweep :type Boolean) (SweepResult :type Hit%20Result%20Structure%20%28by%20ref%29))
  ;[1 1 1] enemyにぶつかると爆発して真っ黒になりダメージアクションをとる
  (bind _asbp_enemy (Utilities|Casting|CastToBP_enemy OtherActor))
  (if (stale Input|KeyboardEvents|Z _output_get)
    (Variables|Default|SetdamageFlag true)
    (Effects|SpawnEmitteratLocation "/Game/StarterContent/Particles/P_Explosion.P_Explosion" (Transformation|GetWorldLocation (Variables|Character|GetMesh)) "0, 0, 0" "5.000000,5.000000,5.000000" false)
    (bind _asbp_unitychan (Utilities|Casting|CastToBP_unitychan (Game|Player|GetPlayerPawn 0)))
    (Game|Damage|ApplyDamage _asbp_unitychan 1.0 0 0)
    (Rendering|Material|SetMaterial (Variables|Character|GetMesh) 0 "/Game/texture/hair_damage.hair_damage")
    (Rendering|Material|SetMaterial (Variables|Character|GetMesh) 1 "/Game/texture/body_damage.body_damage")
    (Rendering|Material|SetMaterial (Variables|Character|GetMesh) 2 "/Game/texture/skin_damage.skin_damage")
    (Rendering|Material|SetMaterial (Variables|Character|GetMesh) 4 "/Game/texture/face_damage.face_damage")
    (Rendering|Material|SetMaterial (Variables|Character|GetMesh) 8 "/Game/texture/eyeline_damage.eyeline_damage")
    (Utilities|FlowControl|Delay 3.0)
    (Variables|Default|SetdamageFlag false)
    (Utilities|FlowControl|Delay 5.0)
    (Rendering|Material|SetMaterial (Variables|Character|GetMesh) 0 "/Game/texture/hair_01_Mat.hair_01_Mat")
    (Rendering|Material|SetMaterial (Variables|Character|GetMesh) 1 "/Game/texture/body_01_Mat.body_01_Mat")
    (Rendering|Material|SetMaterial (Variables|Character|GetMesh) 2 "/Game/texture/skin_01_Mat.skin_01_Mat")
    (Rendering|Material|SetMaterial (Variables|Character|GetMesh) 4 "/Game/texture/face_00_Mat.face_00_Mat")
    (Rendering|Material|SetMaterial (Variables|Character|GetMesh) 8 "/Game/texture/eyeline_00_Mat.eyeline_00_Mat")
    (else
      (Utilities|FlowControl|Delay 2.0)
      (Variables|Default|SetdamageFlag2 true))))

(event EventBeginPlay)

(event Collision|EventActorBeginOverlap
  (params (OtherActor :type Actor%20Object%20Reference)))

(event EventTick
  (params (DeltaSeconds :type Float%20%28single-precision%29)))

(event Game|Damage|EventAnyDamage
  (params (Damage :type Float%20%28single-precision%29) (DamageType :type Damage%20Type%20Object%20Reference) (InstigatedBy :type Controller%20Object%20Reference) (DamageCauser :type Actor%20Object%20Reference))
  ;[1 1 1] ダメージ処理
  (Variables|Default|SetHP (- (Variables|Default|GetHP) Damage)))

(event Input|KeyboardEvents|Z
  (params (Key :type Key%20Structure))
  ;[1 1 1] enemyにぶつかると爆発して真っ黒になりダメージアクションをとる
  (:Pressed
    (bind _output_get (Variables|Default|SetdamageFlag2 false))))

(fn ConstructionScript)