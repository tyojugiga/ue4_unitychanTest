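; BP_enemy3 is an enemy built around a Destructible component that chases the player's BP_unitychan.
; While the component is valid, Tick feeds movement input along the horizontal direction toward the player's mesh.
; Overlapping BP_unitychan shatters the Destructible with radius damage, ragdolls the player and applies damage.
; A BP_fire hit shatters it with a weaker impulse; in both cases the component is destroyed after a short delay.
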(event OnComponentBeginOverlap(Destructible)
  (params (OverlappedComponent :type Primitive%20Component%20Object%20Reference) (OtherActor :type Actor%20Object%20Reference) (OtherComp :type Primitive%20Component%20Object%20Reference) (OtherBodyIndex :type Integer) (bFromSweep :type Boolean) (SweepResult :type Hit%20Result%20Structure%20%28by%20ref%29))
  (Utilities|FlowControl|Sequence
    (:then_0
      ;[1 1 1] unitychanをラグドール化させる
      (bind _asbp_unitychan (Utilities|Casting|CastToBP_unitychan OtherActor))
      (Class|DestructibleComponent|ApplyRadiusDamage (Variables|Default|GetDestructible) 1e+02 (Transformation|GetWorldLocation (Variables|Default|GetDestructible)) 1e+02 1e+04 false)
      (bind _asbp_unitychan_2 (Utilities|Casting|CastToBP_unitychan OtherActor))
      (Collision|SetCollisionEnabled (Variables|/Script/Engine.Character|GetCapsuleComponent _asbp_unitychan_2) "NoCollision")
      (Class|SkeletalMeshComponent|SetAllBodiesSimulatePhysics (Variables|/Script/Engine.Character|GetMesh _asbp_unitychan_2) true)
      (Game|Damage|ApplyDamage _asbp_unitychan_2 1e+02 0 0)
      (Utilities|FlowControl|Delay 1.5)
      (Components|DestroyComponent (Variables|Default|GetDestructible)))
    (:then_1
      ;[1 1 1] unitychanに攻撃されると砕ける
      (bind _asbp_fire (Utilities|Casting|CastToBP_fire OtherActor))
      (Class|DestructibleComponent|ApplyRadiusDamage (Variables|Default|GetDestructible) 1e+02 (Transformation|GetWorldLocation (Variables|Default|GetDestructible)) 1e+02 1e+03 false)
      (Utilities|FlowControl|Delay 1.5)
      (Components|DestroyComponent (Variables|Default|GetDestructible)))))

(event EventBeginPlay)

(event Collision|EventActorBeginOverlap
  (params (OtherActor :type Actor%20Object%20Reference)))

(event EventTick
  (params (DeltaSeconds :type Float%20%28single-precision%29))
  ;[1 1 1] unitychan追跡
  (Utilities|IsValid (Variables|Default|GetDestructible)
    (:Is%20Valid
      (bind _asbp_unitychan (Utilities|Casting|CastToBP_unitychan (Game|GetPlayerCharacter 0)))
      (Pawn|Input|AddMovementInput (Math|Vector|MakeVector (.X (Math|Vector|BreakVector (- (Transformation|GetWorldLocation (Variables|/Script/Engine.Character|GetMesh _asbp_unitychan)) (Transformation|GetWorldLocation (Variables|Default|GetDestructible))))) (.Y (Math|Vector|BreakVector (- (Transformation|GetWorldLocation (Variables|/Script/Engine.Character|GetMesh _asbp_unitychan)) (Transformation|GetWorldLocation (Variables|Default|GetDestructible))))) 0.0) 1.0 false))))

(fn ConstructionScript)