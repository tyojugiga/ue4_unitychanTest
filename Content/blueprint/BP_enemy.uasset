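; Enemy pawn that chases the BP_unitychan player and shatters when kicked by or bumped into that character.
; Every Tick, while its Destructible component is valid, it adds movement input toward the player's mesh on the horizontal plane.
; A Sphere overlap with the player fractures the Destructible through radius damage at its own location, then destroys both components after a short delay, leaving the actor itself alive.
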(event OnComponentBeginOverlap(Sphere)
  (params (OverlappedComponent :type Primitive%20Component%20Object%20Reference) (OtherActor :type Actor%20Object%20Reference) (OtherComp :type Primitive%20Component%20Object%20Reference) (OtherBodyIndex :type Integer) (bFromSweep :type Boolean) (SweepResult :type Hit%20Result%20Structure%20%28by%20ref%29))
  ;[1 1 1] unitychanに回し蹴りされるか、ぶつかると砕ける
  (bind _asbp_unitychan (Utilities|Casting|CastToBP_unitychan OtherActor))
  (Class|DestructibleComponent|ApplyRadiusDamage (Variables|Default|GetDestructible) 1e+02 (Transformation|GetWorldLocation (Variables|Default|GetDestructible)) 5e+03 5e+03 false)
  (Utilities|FlowControl|Delay 1.5)
  (Components|DestroyComponent (Variables|Default|GetDestructible))
  (Components|DestroyComponent (Variables|Default|GetSphere)))

(event EventBeginPlay)

(event Collision|EventActorBeginOverlap
  (params (OtherActor :type Actor%20Object%20Reference)))

(event EventTick
  (params (DeltaSeconds :type Float%20%28single-precision%29))
  ;[1 1 1] unitychan追跡
  (Utilities|IsValid (Variables|Default|GetDestructible)
    (:Is%20Valid
      (bind _asbp_unitychan (Utilities|Casting|CastToBP_unitychan (Game|GetPlayerCharacter 0)))
      (Pawn|Input|AddMovementInput (Math|Vector|MakeVector (.X (Math|Vector|BreakVector (- (Transformation|GetWorldLocation (Variables|/Script/Engine.Character|GetMesh _asbp_unitychan)) (Transformation|GetWorldLocation (Variables|Default|GetDestructible))))) (.Y (Math|Vector|BreakVector (- (Transformation|GetWorldLocation (Variables|/Script/Engine.Character|GetMesh _asbp_unitychan)) (Transformation|GetWorldLocation (Variables|Default|GetDestructible))))) 0.0) 1.0 false))))

(fn ConstructionScript)