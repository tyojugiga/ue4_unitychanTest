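; BP_enemy2 is a falling hazard that drops when the player character BP_unitychan passes beneath it and shatters when it lands on her.
; A Box trigger enables physics simulation on the Destructible component, then destroys itself so the drop fires only once.
; When the Destructible overlaps BP_unitychan, it applies radius damage to itself to fracture, then is removed after a short delay.
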(event OnComponentBeginOverlap(Box)
  (params (OverlappedComponent :type Primitive%20Component%20Object%20Reference) (OtherActor :type Actor%20Object%20Reference) (OtherComp :type Primitive%20Component%20Object%20Reference) (OtherBodyIndex :type Integer) (bFromSweep :type Boolean) (SweepResult :type Hit%20Result%20Structure%20%28by%20ref%29))
  ;[1 1 1] unitychanが下に入ると落下する
  (bind _asbp_unitychan (Utilities|Casting|CastToBP_unitychan OtherActor))
  (Physics|SetSimulatePhysics (Variables|Default|GetDestructible) true)
  (Components|DestroyComponent (Variables|Default|GetBox)))

(event OnComponentBeginOverlap(Destructible)
  (params (OverlappedComponent :type Primitive%20Component%20Object%20Reference) (OtherActor :type Actor%20Object%20Reference) (OtherComp :type Primitive%20Component%20Object%20Reference) (OtherBodyIndex :type Integer) (bFromSweep :type Boolean) (SweepResult :type Hit%20Result%20Structure%20%28by%20ref%29))
  ;[1 1 1] unitychanの上に落ちると砕ける
  (bind _asbp_unitychan (Utilities|Casting|CastToBP_unitychan OtherActor))
  (Class|DestructibleComponent|ApplyRadiusDamage (Variables|Default|GetDestructible) 1e+02 (Transformation|GetWorldLocation (Variables|Default|GetDestructible)) 1e+02 5e+02 false)
  (Utilities|FlowControl|Delay 1.5)
  (Components|DestroyComponent (Variables|Default|GetDestructible)))

(event EventBeginPlay)

(event Collision|EventActorBeginOverlap
  (params (OtherActor :type Actor%20Object%20Reference)))

(event EventTick
  (params (DeltaSeconds :type Float%20%28single-precision%29)))

(fn ConstructionScript)